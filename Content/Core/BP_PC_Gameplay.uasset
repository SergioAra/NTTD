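; BP_PC_Gameplay is the gameplay player controller, handling input mode and the pause menu.
; BeginPlay sets game-only input with the cursor hidden.
; PausetheGame lazily creates and caches the pause widget, adds it to the viewport, and switches to UI-only input with a visible cursor.
; UnPausetheGame removes the widget and restores game input; neither event sets the engine's paused state.
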(event `self.ReceiveBeginPlay`
  (`WidgetBlueprintLibrary.SetInputMode_GameOnly` self)
  (set `self.bShowMouseCursor` false))

(event `self.BP_PauseTheGame`
  (params (CurrentPausedState :type Boolean))
  (bind _returnvalue (`GameplayStatics.GetPlayerController` 0))
  (`/Engine/EditorBlueprintResources/StandardMacros.IsValid` (`self.WPauseMenuReference`)
    (:`Is Valid`
      _)
    (:`Is Not Valid`
      (bind _returnvalue_2 (`|CreateWidget` "/Game/UI/PauseMenu/W_PauseMenu.W_PauseMenu_C"))
      (bind _output_get (set `self.WPauseMenuReference` _returnvalue_2))))
  (`UserWidget.AddToViewport` _output_get 0)
  (`WidgetBlueprintLibrary.SetInputMode_UIOnlyEx` _returnvalue null)
  (set `PlayerController.bShowMouseCursor` true _returnvalue))

(event `self.BP_UnPauseTheGame`
  (params (CurrentPausedState :type Boolean))
  (bind _returnvalue (`GameplayStatics.GetPlayerController` 0))
  (bind _wpausemenureference (`self.WPauseMenuReference`))
  (`/Engine/EditorBlueprintResources/StandardMacros.IsValid` _wpausemenureference
    (:`Is Valid`
      (`Widget.RemoveFromParent` _wpausemenureference)
      (`WidgetBlueprintLibrary.SetInputMode_GameOnly` _returnvalue)
      (set `PlayerController.bShowMouseCursor` false _returnvalue))))

(fn `UserConstructionScript`)