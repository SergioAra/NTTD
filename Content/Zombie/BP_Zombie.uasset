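; Zombie enemy pawn that attacks with random left or right arm montages, using a separate set when heavily damaged.
; Non-lethal hits flag its AI controller and report a damage sense event, while lethal ones add score to the instigating TopDownCharacter.
; Death ragdolls the mesh, destroys the AI controller and hand colliders, then after a delay removes the zombie from its spawner's list and destroys it.
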(event `self.ReceiveBeginPlay`
  (bind _asaic_zombie_enemy (cast `/Game/Zombie/AI/AIC_ZombieEnemy` (`self.GetController`)))
  (set `self.AICZombieEnemyReference` _asaic_zombie_enemy))

(event `self.ReceiveTick`
  (params (DeltaSeconds :type "Float (single-precision)")))

(event `self.BP_Death`
  (bind _returnvalue (`AIBlueprintHelperLibrary.GetAIController` self))
  (`PrimitiveComponent.SetSimulatePhysics` (`self.Mesh`) true)
  (`CharacterMovementComponent.DisableMovement` (`self.CharacterMovement`))
  (`ActorComponent.Deactivate` (`AIController.ActionsComp` _returnvalue))
  (`self.K2_DestroyActor` _returnvalue)
  (`ActorComponent.K2_DestroyComponent` (`self.RightHandCollider`))
  (`ActorComponent.K2_DestroyComponent` (`self.LeftHandCollider`))
  (`KismetSystemLibrary.Delay` 4.0)
  ;[1 1 1] Remove enemy from spawner list
  (`KismetArrayLibrary.Array_RemoveItem` (`/Game/EnemySpawner/EnemySpawner.SpawnedList` (`self.Spawner`)) self)
  (`self.K2_DestroyActor`))

(event `self.BP_OnHealthChange`
  (params (CurrentHealthComponent :type "NTTD_HealthComponent Object Reference") (DamagedActor :type "Actor Object Reference") (Damage :type "Float (single-precision)") (DamageType :type "DamageType Object Reference") (InstigatedBy :type "Controller Object Reference") (DamageCauser :type "Actor Object Reference"))
  (if (`NTTD_HealthComponent.GetIsDead` CurrentHealthComponent)
    (bind _astop_down_character (cast `/Game/TopDownCPP/Blueprints/TopDownCharacter` (`Controller.K2_GetPawn` InstigatedBy)))
    (`NTTDCharacter.IncremetScore` _astop_down_character (`self.ScoreValue`))
    (else
      (`|ExecutionSequence`
        (:`then_0`
          (bind _aiczombieenemyreference (`self.AICZombieEnemyReference`)
            (:`then`
              (set `/Game/Zombie/AI/AIC_ZombieEnemy.bIsDamaged` true _aiczombieenemyreference))
            (:`else`)))
        (:`then_1`
          (`AISense_Damage.ReportDamageEvent` self DamageCauser Damage (`self.K2_GetActorLocation` DamageCauser)))))))

(event `CustomBP_Attack`
  (bind _returnvalue (== (`KismetMathLibrary.RandomIntegerInRange` 0 1) 0))
  ;[1 1 1] Attack Logic
  (if (not (`self.bIsAttacking`))
    (set `self.bIsAttacking` true)
    (if (`self.bIsHeavilyDamaged`)
      (if _returnvalue
        (set `self.AttackMontageToPlay` (`self.HeavilyDamagedAttackRightArmMontage`))
        (else
          (set `self.AttackMontageToPlay` (`self.HeavilyDamagedAttackLeftArmMontage`))))
      (elif _returnvalue
        (set `self.AttackMontageToPlay` (`self.NormalAttackRightArmMontage`))
        (else
          (set `self.AttackMontageToPlay` (`self.NormalAttackLeftArmMontage`)))))
    (bind _attackmontagetoplay (`self.AttackMontageToPlay`)
      (:`then`
        (`|PlayMontage` (`self.Mesh`) _attackmontagetoplay
          (:`OnCompleted`
            (set `self.bIsAttacking` false))))
      (:`else`))))

(fn `BP_Attack`
  (`self.CustomBP_Attack`))

(fn `UserConstructionScript`)